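; VR player pawn that drives a full-body skeletal mesh from the headset camera.
; BeginPlay enables stereo with floor tracking, finds the "Attacker"-tagged Boris character and creates a damage widget.
; Each tick, camera movement or yaw past thresholds sets an offset body target, which the mesh then lerps toward at a motion-derived speed.
; Sight, Sound and Framedrop switches are stubs; the pause-based frame-drop and foot-tracking logic is disconnected.
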(event EventBeginPlay
  (Development|ExecuteConsoleCommand "stereo on" 0)
  (Class|HeadMountedDisplayFunctionLibrary|SetTrackingOrigin "Floor")
  (bind _outactors (Actor|GetAllActorswithTag "Attacker"))
  (for _array_element _outactors
    (bind _output_get (Variables|Default|SetAttacker _array_element))
    (bind _asmy_boris_player_character (Utilities|Casting|CastToMY_BorisPlayerCharacter _output_get))
    (Variables|Default|SetAs%20MY%20Boris%20Player%20Character _asmy_boris_player_character)
    (bind _returnvalue (UserInterface|CreateWidget "/Game/TestField/DamagedUI.DamagedUI_C"))
    (Variables|Default|SetDamageUI _returnvalue)))

(event Collision|EventActorBeginOverlap
  (params (OtherActor :type Actor%20Object%20Reference)))

(event EventTick
  (params (DeltaSeconds :type Float%20%28single-precision%29))
  (CallFunction|CalculteMovement)
  (if (Variables|Default|GetSight)
    (CallFunction|SightDifference)
    (elif (Variables|Default|GetSound)
      (CallFunction|TempoChange)
      (elif (Variables|Default|GetFramedrop)
        _))))

(event Input|ActionEvents|InputActionchase
  (params (Key :type Key%20Structure)))

(fn ConstructionScript
  (Transformation|DetachFromComponent (Variables|Default|GetSkeletalMesh) "KeepRelative" "KeepRelative" "KeepRelative" true))

(fn CalculteMovement
  (bind (_rotation _location) (CallFunction|GetBodyOffset))
  (bind _camera (Variables|Default|GetCamera))
  (bind _returnvalue (Transformation|GetWorldTransform _camera))
  (Transformation|SetRelativeScale3D (Variables|Default|GetSkeletalMesh) "1.000000,1.000000,1.000000")
  (bind _output_get (LocalVariables|SetCurrent%20Camera%20Postion (Math|Transform|MakeTransform (Math|Vector|MakeVector (.x (.location _returnvalue)) (.y (.location _returnvalue)) 0.0) (Math|Rotator|MakeRotator 0.0 0.0 (.yaw (.rotation _returnvalue))) "1,1,1")))
  (bind _distance_moved (CallFunction|GetDistanceMoved (.x (.location _output_get)) (.y (.location _output_get))))
  (LocalVariables|SetDistance%20Moved _distance_moved)
  (bind _distance_rotated (CallFunction|GetDistanceRotated (.rotation _output_get)))
  (LocalVariables|SetDistance%20Rotated _distance_rotated)
  (Utilities|FlowControl|Sequence
    (:then_0
      ;[1 1 1] Rotation
      (if (or (> (LocalVariables|GetDistance%20Moved) (Variables|Default|GetMovement%20Threshold)) (> (LocalVariables|GetDistance%20Rotated) (Variables|Default|GetRotation%20Threshold)))
        (Variables|Position|SetBody%20Target%20Position (Math|Transform|MakeTransform _location _rotation "1,1,1"))
        (Variables|Position|SetMovement%20Direction (Utilities|GetDirection (LocalVariables|GetCurrent%20Camera%20Postion)))
        (Variables|Position|SetLast%20Camera%20Postion (LocalVariables|GetCurrent%20Camera%20Postion))
        (Variables|Position|SetMovement%20Speed (/ (/ (+ (LocalVariables|GetDistance%20Moved) (LocalVariables|GetDistance%20Rotated)) 2e+03) (Utilities|Time|GetWorldDeltaSeconds)))
        (elif (== (Variables|Position|GetBody%20Current%20Postion) (Variables|Position|GetBody%20Target%20Position))
          (Variables|Position|SetMovement%20Speed 0.0)
          (Variables|Position|SetMovement%20Direction 0.0)
          (Variables|Position|SetAlpha 0.0)
          (else
            (Variables|Position|SetAlpha (Math|Interpolation|FInterptoConstant (Variables|Position|GetAlpha) 1.0 (Utilities|Time|GetWorldDeltaSeconds) (Variables|Position|GetMovement%20Speed)))
            (bind _output_get_2 (Variables|Position|SetBody%20Current%20Postion (Math|Transform|Lerp(Transform) (Variables|Position|GetBody%20Current%20Postion) (Variables|Position|GetBody%20Target%20Position) (Variables|Position|GetAlpha))))
            (Transformation|SetWorldLocationAndRotation (Variables|Default|GetSkeletalMesh) (.location _output_get_2) (.rotation _output_get_2) false false)))))))

(fn GetDistanceMoved
  (params (Current%20X :type Float%20%28single-precision%29) (Current%20Y :type Float%20%28single-precision%29))
  (bind _last_camera_postion (Variables|Position|GetLast%20Camera%20Postion))
  (return (Math|Vector|Distance(Vector) (Math|Vector|MakeVector Current%20X Current%20Y 0.0) (Math|Vector|MakeVector (.x (.location _last_camera_postion)) (.y (.location _last_camera_postion)) 0.0))))

(fn GetDistanceRotated
  (params (Current%20Rotation :type Rotator))
  (return (Math|Float|Absolute(Float) (- (.yaw Current%20Rotation) (.yaw (.rotation (Variables|Position|GetLast%20Camera%20Postion)))))))

(fn GetBodyRotationfromHMD
  (return (Math|Rotator|MakeRotator 0.0 0.0 (- (.yaw (.rotation (Transformation|GetWorldTransform (Variables|Default|GetCamera)))) 9e+01))))

(fn GetBodyOffset
  (bind _camera (Variables|Default|GetCamera))
  (bind _returnvalue (Transformation|GetWorldTransform _camera))
  (bind _returnvalue_2 (- (.yaw (.rotation _returnvalue)) 9e+01))
  (bind _returnvalue_3 (Math|Rotator|MakeRotator 0.0 0.0 _returnvalue_2))
  (bind _returnvalue_4 (Math|Vector|GetRightVector _returnvalue_3))
  (bind _returnvalue_5 (* _returnvalue_4 -20))
  (bind _returnvalue_6 (+ (.location _returnvalue) _returnvalue_5))
  (return _returnvalue_3 (Math|Vector|MakeVector (.x _returnvalue_6) (.y _returnvalue_6) (- (.z _returnvalue_6) 1.7e+02))))

(fn SightDifference)

(fn TempoChange)

(fn GenerateFrame-drop
  (Class|Actor|SetTickablewhenPaused true)
  (Game|SetGamePaused true))