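; VR player pawn with a skeletal body that follows the headset, apparently for an experiment with left/right judgement input.
; Each tick, CalculteMovement derives speed from camera movement and yaw past thresholds, lerping the detached mesh toward an offset below the HMD.
; A right-hand widget pointer handles UI clicks, judge inputs set Correct, and a blood overlay fades after hits.
; Both foot controllers' positions accumulate every tick and save to a text file on EndPlay.
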(event Custom|Widget%20Interaction
  (bind _skeletalmesh (Variables|Default|GetSkeletalMesh))
  (Transformation|SetWorldLocationAndRotation (Variables|Default|GetWidgetInteraction) (Transformation|GetSocketLocation _skeletalmesh "hand_r") (Math|Rotator|CombineRotators "180.000000,0.000000,0.000000" (Transformation|GetSocketRotation _skeletalmesh "hand_r")) false false))

(event EventBeginPlay
  (Utilities|FlowControl|Sequence
    (:then_0
      (Development|ExecuteConsoleCommand "stereo on" 0)
      (Class|HeadMountedDisplayFunctionLibrary|SetTrackingOrigin "Floor")
      (bind _returnvalue (UserInterface|CreateWidget "/Game/BloodOverlayWidget.BloodOverlayWidget_C"))
      (UserInterface|Viewport|AddtoViewport _returnvalue 0)
      (Variables|Default|SetBloodOverlay _returnvalue))
    (:then_1
      (bind _returnvalue_2 (UserInterface|CreateWidget "/Game/TextBlockWidget.TextBlockWidget_C"))
      (UserInterface|Viewport|AddtoViewport _returnvalue_2 0))))

(event Collision|EventActorBeginOverlap
  (params (OtherActor :type Actor%20Object%20Reference)))

(event EventTick
  (params (DeltaSeconds :type Float%20%28single-precision%29))
  (bind _bloodoverlay (Variables|Default|GetBloodOverlay))
  (bind _colorandopacity (Variables|/Script/UMG.UserWidget|GetColorAndOpacity _bloodoverlay))
  (Variables|Default|SetLFoot (Utilities|String|Append (Variables|Default|GetLFoot) (Utilities|String|ToString(Vector) (Transformation|GetWorldLocation (Variables|Default|GetMotionController_LFoot))) " 
" (Utilities|String|ToString(Vector) (Transformation|GetWorldLocation (Variables|Default|GetMotionController_RFoot))) " 
"))
  (CallFunction|CalculteMovement)
  (CallFunction|WidgetInteraction)
  ;[1 1 1] hit
  (if (Variables|Default|GetIsHit)
    (Appearance|SetColorandOpacity _bloodoverlay (Math|Color|MakeColor (.r _colorandopacity) (.g _colorandopacity) (.b _colorandopacity) (- (.a _colorandopacity) 0.01)) :!class /Script/UMG.UserWidget)
    (if (<= (.a (Variables|/Script/UMG.UserWidget|GetColorAndOpacity (Variables|Default|GetBloodOverlay))) 0.0)
      (Variables|Default|SetIsHit false))))

(event EventEndPlay
  (params (EndPlayReason :type EEndPlayReason%20Enum :default "Destroyed"))
  (Class|PrintUtilityLibrary|FileSaveString (Variables|Default|GetLFoot) "lfoot.txt"))

(event Input|ActionEvents|InputActionJudgeL
  (params (Key :type Key%20Structure :default "None"))
  (:Pressed
    (Variables|Default|SetCorrect 1)))

(event Input|ActionEvents|InputActionselectUI
  (params (Key :type Key%20Structure :default "None"))
  (bind _widgetinteraction (Variables|Default|GetWidgetInteraction))
  (:Pressed
    (Class|WidgetInteractionComponent|PressPointerKey _widgetinteraction "LeftMouseButton"))
  (:Released
    (Class|WidgetInteractionComponent|ReleasePointerKey _widgetinteraction "LeftMouseButton")))

(event Input|ActionEvents|InputActionJudgeR
  (params (Key :type Key%20Structure :default "None"))
  (:Pressed
    (Variables|Default|SetCorrect 2)))

(fn ConstructionScript
  (Transformation|DetachFromComponent (Variables|Default|GetSkeletalMesh) "KeepRelative" "KeepRelative" "KeepRelative" true))

(fn CalculteMovement
  (bind (_rotation _location) (CallFunction|GetBodyOffset))
  (bind _camera (Variables|Default|GetCamera))
  (bind _returnvalue (Transformation|GetWorldTransform _camera))
  (Transformation|SetRelativeScale3D (Variables|Default|GetSkeletalMesh) "1.000000,1.000000,1.000000")
  (bind _output_get (LocalVariables|SetCurrent%20Camera%20Postion (Math|Transform|MakeTransform (Math|Vector|MakeVector (.x (.location _returnvalue)) (.y (.location _returnvalue)) 0.0) (Math|Rotator|MakeRotator 0.0 0.0 (.yaw (.rotation _returnvalue))) "1,1,1")))
  (bind _distance_moved (CallFunction|GetDistanceMoved (.x (.location _output_get)) (.y (.location _output_get))))
  (LocalVariables|SetDistance%20Moved _distance_moved)
  (bind _distance_rotated (CallFunction|GetDistanceRotated (.rotation _output_get)))
  (LocalVariables|SetDistance%20Rotated _distance_rotated)
  (Utilities|FlowControl|Sequence
    (:then_0
      ;[1 1 1] Rotation
      (if (or (> (LocalVariables|GetDistance%20Moved) (Variables|Default|GetMovement%20Threshold)) (> (LocalVariables|GetDistance%20Rotated) (Variables|Default|GetRotation%20Threshold)))
        (Variables|Position|SetBody%20Target%20Position (Math|Transform|MakeTransform _location _rotation "1,1,1"))
        (Variables|Position|SetMovement%20Direction (Utilities|GetDirection (LocalVariables|GetCurrent%20Camera%20Postion)))
        (Variables|Position|SetLast%20Camera%20Postion (LocalVariables|GetCurrent%20Camera%20Postion))
        (Variables|Position|SetMovement%20Speed (/ (/ (+ (LocalVariables|GetDistance%20Moved) (LocalVariables|GetDistance%20Rotated)) 2e+03) (Utilities|Time|GetWorldDeltaSeconds)))
        (elif (== (Variables|Position|GetBody%20Current%20Postion) (Variables|Position|GetBody%20Target%20Position))
          (Variables|Position|SetMovement%20Speed 0.0)
          (Variables|Position|SetMovement%20Direction 0.0)
          (Variables|Position|SetAlpha 0.0)
          (else
            (Variables|Position|SetAlpha (Math|Interpolation|FInterptoConstant (Variables|Position|GetAlpha) 1.0 (Utilities|Time|GetWorldDeltaSeconds) (Variables|Position|GetMovement%20Speed)))
            (bind _output_get_2 (Variables|Position|SetBody%20Current%20Postion (Math|Transform|Lerp(Transform) (Variables|Position|GetBody%20Current%20Postion) (Variables|Position|GetBody%20Target%20Position) (Variables|Position|GetAlpha))))
            (Transformation|SetWorldLocationAndRotation (Variables|Default|GetSkeletalMesh) (.location _output_get_2) (.rotation _output_get_2) false false)))))
    (:then_1
      ;;[1 1 1] Z for IK
      (Transformation|SetWorldLocationAndRotation (Variables|Default|GetSkeletalMesh) (Math|Vector|MakeVector (.x (.location (Variables|Position|GetBody%20Current%20Postion))) (.y (.location (Variables|Position|GetBody%20Current%20Postion))) (.z (.Location (CallFunction|GetBodyOffset)))) (.rotation (Variables|Position|GetBody%20Current%20Postion)) false false))))

(fn GetDistanceMoved
  (params (Current%20X :type Float%20%28single-precision%29) (Current%20Y :type Float%20%28single-precision%29))
  (bind _last_camera_postion (Variables|Position|GetLast%20Camera%20Postion))
  (return (Math|Vector|Distance(Vector) (Math|Vector|MakeVector Current%20X Current%20Y 0.0) (Math|Vector|MakeVector (.x (.location _last_camera_postion)) (.y (.location _last_camera_postion)) 0.0))))

(fn GetDistanceRotated
  (params (Current%20Rotation :type Rotator))
  (return (Math|Float|Absolute(Float) (- (.yaw Current%20Rotation) (.yaw (.rotation (Variables|Position|GetLast%20Camera%20Postion)))))))

(fn GetBodyRotationfromHMD
  (return (Math|Rotator|MakeRotator 0.0 0.0 (- (.yaw (.rotation (Transformation|GetWorldTransform (Variables|Default|GetCamera)))) 9e+01))))

(fn GetBodyOffset
  (bind _camera (Variables|Default|GetCamera))
  (bind _returnvalue (Transformation|GetWorldTransform _camera))
  (bind _returnvalue_2 (- (.yaw (.rotation _returnvalue)) 9e+01))
  (bind _returnvalue_3 (Math|Rotator|MakeRotator 0.0 0.0 _returnvalue_2))
  (bind _returnvalue_4 (Math|Vector|GetRightVector _returnvalue_3))
  (bind _returnvalue_5 (* _returnvalue_4 -20))
  (bind _returnvalue_6 (+ (.location _returnvalue) _returnvalue_5))
  (return _returnvalue_3 (Math|Vector|MakeVector (.x _returnvalue_6) (.y _returnvalue_6) (- (.z _returnvalue_6) 175.0))))