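; HackerGameInstance is a Game Instance that generates and holds the randomized passwords for a hacking game.
; Separate events append random digits for the login and AGWG passwords, set a one-digit AGWG user number, and fill the ShapePassword array with random shape enums.
; The second shape password maps each of three enum values to a random digit, then MakeShapePassword2 joins those digits in a fixed seven-symbol order as text.
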(event Custom|SetShapePassword2
  (Variables|Default|SetShapePassword2_Map (Utilities|Map|MakeMap "NewEnumerator0" (Math|Random|RandomIntegerinRange 3 8) "NewEnumerator1" (Math|Random|RandomIntegerinRange 3 8) "NewEnumerator2" (Math|Random|RandomIntegerinRange 3 8)))
  (Variables|Default|SetShapePassword2 (CallFunction|MakeShapePassword2)))

(event Custom|Set%20AWGW
  (Variables|Default|SetAGWGUserNumber (Utilities|String|ToString(Integer) (Math|Random|RandomInteger 10)))
  ;[1 1 1] password
  (for _index (range 0 3)
    (Variables|Default|SetAGWGPassword (Utilities|String|Append (Variables|Default|GetAGWGPassword) (Utilities|String|ToString(Integer) (Math|Random|RandomInteger 10))))))

(event Custom|Set%20LoginPassword
  (for _index (range 0 3)
    (Variables|Default|SetloginPassword (Utilities|String|Append (Variables|Default|GetloginPassword) (Utilities|String|ToString(Integer) (Math|Random|RandomInteger 10))))))

(event Custom|SetShapePassword
  (for (_ _array_index) (Variables|Default|GetShapePassword)
    (switch int (Math|Random|RandomInteger 3)
      (:0
        (Utilities|Array|SetArrayElem (Variables|Default|GetShapePassword) _array_index "NewEnumerator0"))
      (:1
        (Utilities|Array|SetArrayElem (Variables|Default|GetShapePassword) _array_index "NewEnumerator1"))
      (:2
        (Utilities|Array|SetArrayElem (Variables|Default|GetShapePassword) _array_index "NewEnumerator2")))))

(fn MakeShapePassword2
  (return (Utilities|Text|ToText(String) (Utilities|String|Append (Utilities|String|ToString(Integer) (.Value (Utilities|Map|Find (Variables|Default|GetShapePassword2_Map) "NewEnumerator1"))) (Utilities|String|ToString(Integer) (.Value (Utilities|Map|Find (Variables|Default|GetShapePassword2_Map) "NewEnumerator1"))) (Utilities|String|ToString(Integer) (.Value (Utilities|Map|Find (Variables|Default|GetShapePassword2_Map) "NewEnumerator2"))) (Utilities|String|ToString(Integer) (.Value (Utilities|Map|Find (Variables|Default|GetShapePassword2_Map) "NewEnumerator0"))) (Utilities|String|ToString(Integer) (.Value (Utilities|Map|Find (Variables|Default|GetShapePassword2_Map) "NewEnumerator1"))) (Utilities|String|ToString(Integer) (.Value (Utilities|Map|Find (Variables|Default|GetShapePassword2_Map) "NewEnumerator0"))) (Utilities|String|ToString(Integer) (.Value (Utilities|Map|Find (Variables|Default|GetShapePassword2_Map) "NewEnumerator0")))))))