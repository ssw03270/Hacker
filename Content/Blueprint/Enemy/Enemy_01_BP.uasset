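; Enemy actor that faces the player and eases toward a Target each tick, setting a walk flag.
; When its post-spawn timer expires, it attacks: applies a GameSystem score penalty, flags either first-person or VR player as hit with blood overlay, and self-destructs.
; Once not live, it topples over, then destroys itself.
; A Gaussian curve over the timer shapes EnemyGenerator's walk-sound volume, which stops on attack or death.
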(event EventBeginPlay
  (CallFunction|LookPlayer))

(event Collision|EventActorBeginOverlap
  (params (OtherActor :type Actor%20Object%20Reference)))

(event EventTick
  (params (DeltaSeconds :type Float%20%28single-precision%29))
  (Utilities|FlowControl|Sequence
    (:then_0
      (if (Variables|Default|GetIsLive)
        (CallFunction|LookPlayer)))
    (:then_1
      (if (and (CallFunction|CheckAttackPlayerAble) (Variables|Default|GetIsLive))
        (CallFunction|AttackPlayer)))
    (:then_2
      (if (not (Variables|Default|GetIsLive))
        (CallFunction|Die)))
    (:then_3
      (if (Variables|Default|GetIsLive)
        (CallFunction|MovetoTarget)))
    (:then_4
      (if (Variables|Default|GetIsLive)
        (CallFunction|SetAnimationState)))
    (:then_5
      (if (Variables|Default|GetIsLive)
        (CallFunction|SetFootSound)))))

(fn ConstructionScript)

(fn LookPlayer
  (Variables|Default|SetFaceDirection (Math|Rotator|MakeRotator 0.0 0.0 (+ (.Yaw (Math|Rotator|BreakRotator (Math|Rotator|FindLookatRotation (Transformation|GetActorLocation) (Transformation|GetActorLocation (Game|Player|GetPlayerPawn 0))))) -9e+01)))
  (Transformation|SetActorRotation (Variables|Default|GetFaceDirection)))

(fn CheckAttackPlayerAble
  (Variables|Default|SetAfterSpawnTime (+ (Variables|Default|GetAfterSpawnTime) (Utilities|Time|GetWorldDeltaSeconds)))
  (return (> (Variables|Default|GetAfterSpawnTime) (Variables|Default|GetAfterSpawnTimeMax))))

(fn AttackPlayer
  (bind _returnvalue (Game|Player|GetPlayerPawn 0))
  (bind _returnvalue_2 (Actor|GetActorOfClass (Variables|Default|GetGameSystem)))
  (bind _asgame_system (Utilities|Casting|CastToGameSystem _returnvalue_2))
  (Default|AddObstructionScore _asgame_system (Variables|Default|GetAttackPenalty))
  (bind _returnvalue_3 (Actor|GetActorOfClass (Variables|Default|GetEnemyGenerator)))
  (bind _asenemy_generator_bp (Utilities|Casting|CastToEnemyGenerator_BP _returnvalue_3))
  (Audio|Components|Audio|Stop (Variables|/Game/Blueprint/Enemy/EnemyGenerator_BP.EnemyGenerator_BP_C|GetWalkSound _asenemy_generator_bp))
  (bind _asfirst_person_character (Utilities|Casting|CastToFirstPersonCharacter _returnvalue)
    (:then
      (Variables|/Game/FirstPersonBP/Blueprints/FirstPersonCharacter.FirstPersonCharacter_C|SetIsHit _asfirst_person_character true)
      (Appearance|SetColorandOpacity (Variables|/Game/FirstPersonBP/Blueprints/FirstPersonCharacter.FirstPersonCharacter_C|GetBloodOverlay _asfirst_person_character) "(R=1.000000,G=1.000000,B=1.000000,A=0.200000)" :!class /Script/UMG.UserWidget)
      (Actor|DestroyActor))
    (:CastFailed
      (bind _asbp_vrplayer_man (Utilities|Casting|CastToBP_VRPlayer_Man _returnvalue))
      (Variables|/Game/vrpawn/blueprint/BP_VRPlayer_Man.BP_VRPlayer_Man_C|SetIsHit _asbp_vrplayer_man true)
      (Appearance|SetColorandOpacity (Variables|/Game/vrpawn/blueprint/BP_VRPlayer_Man.BP_VRPlayer_Man_C|GetBloodOverlay _asbp_vrplayer_man) "(R=1.000000,G=1.000000,B=1.000000,A=0.500000)" :!class /Script/UMG.UserWidget)
      (Actor|DestroyActor))))

(fn OnRepGameSystem)

(fn SetLive
  (params (IsLive :type Boolean))
  (Variables|Default|SetIsLive IsLive))

(fn Die
  (bind _returnvalue (Transformation|GetActorRotation))
  (bind _returnvalue_2 (Transformation|GetActorRotation))
  (Transformation|SetActorRotation (Math|Rotator|Lerp(Rotator) (Transformation|GetActorRotation) (Math|Rotator|MakeRotator -9e+01 (.pitch _returnvalue_2) (.yaw _returnvalue_2)) 0.05))
  (if (Math|Rotator|Equal(Rotator) (Transformation|GetActorRotation) (Math|Rotator|MakeRotator -9e+01 (.pitch _returnvalue) (.yaw _returnvalue)) 1e+01)
    (bind _returnvalue_3 (Actor|GetActorOfClass (Variables|Default|GetEnemyGenerator)))
    (bind _asenemy_generator_bp (Utilities|Casting|CastToEnemyGenerator_BP _returnvalue_3))
    (Audio|Components|Audio|Stop (Variables|/Game/Blueprint/Enemy/EnemyGenerator_BP.EnemyGenerator_BP_C|GetWalkSound _asenemy_generator_bp))
    (Actor|DestroyActor)))

(fn MovetoTarget
  (Transformation|SetActorLocation (Math|Vector|Lerp(Vector) (Transformation|GetActorLocation) (Variables|Default|GetTarget) 0.03) false false))

(fn SetAnimationState
  (Variables|Default|SetIsWalk (> (Math|Vector|Distance(Vector) (Transformation|GetActorLocation) (Variables|Default|GetTarget)) 15.0)))

(fn GaussianFunction
  (params (X :type Float%20%28single-precision%29) (Average :type Float%20%28single-precision%29) (Standard%20Deviation :type Float%20%28single-precision%29))
  (return (* (/ 1.0 (Math|Float|Sqrt (* 2.0 (Math|Trig|GetPI) (Math|Float|Square Standard%20Deviation)))) (Class|KismetMathLibrary|Exp (/ (* -1.0 (Math|Float|Square (- X Average))) (* 2.0 (Math|Float|Square Standard%20Deviation)))))))

(fn SetFootSound
  (bind _returnvalue (CallFunction|GaussianFunction (Variables|Default|GetX) 2e+01 2.0))
  (Variables|Default|SetX (+ (Variables|Default|GetX) (* 40 (/ (Utilities|Time|GetWorldDeltaSeconds) (Variables|Default|GetAfterSpawnTimeMax)))))
  (bind _returnvalue_2 (Actor|GetActorOfClass (Variables|Default|GetEnemyGenerator)))
  (bind _asenemy_generator_bp (Utilities|Casting|CastToEnemyGenerator_BP _returnvalue_2))
  (Audio|Components|Audio|SetVolumeMultiplier (Variables|/Game/Blueprint/Enemy/EnemyGenerator_BP.EnemyGenerator_BP_C|GetWalkSound _asenemy_generator_bp) (+ (* 5 _returnvalue) 0.05) :!class /Script/Engine.AudioComponent))