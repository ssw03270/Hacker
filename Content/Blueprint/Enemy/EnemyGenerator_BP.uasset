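; Enemy generator actor that repeatedly spawns an enemy at its own transform on a fixed delay.
; Each Tick it accumulates world delta time and, once the total exceeds the maximum delay, spawns the configured enemy class and resets the timer.
; Spawning also calls an effect hook, which is currently empty.
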(event EventBeginPlay)

(event Collision|EventActorBeginOverlap
  (params (OtherActor :type Actor%20Object%20Reference)))

(event EventTick
  (params (DeltaSeconds :type Float%20%28single-precision%29))
  (if (CallFunction|CheckSpawnDelay)
    (CallFunction|SpawnEnemy)))

(fn ConstructionScript)

(fn SpawnEnemy
  (Game|SpawnActorfromClass (Variables|Default|GetEnemyActor) (Transformation|GetActorTransform) "Undefined" 0 0)
  (Variables|Default|SetDelayCurrent 0.0)
  (CallFunction|EffectGenerator))

(fn CheckSpawnDelay
  (Variables|Default|SetDelayCurrent (+ (Variables|Default|GetDelayCurrent) (Utilities|Time|GetWorldDeltaSeconds)))
  (return (< (Variables|Default|GetDelayMax) (Variables|Default|GetDelayCurrent))))

(fn EffectGenerator)