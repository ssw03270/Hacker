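; UpDownButton is a button Blueprint that nudges a referenced progress bar up or down.
; Its UPorDown event checks that LikedProgressBar is valid, then adds or subtracts a fixed step from the bar's current percent according to the IsUp flag.
; One Blueprint covers both directions, and the graph applies no clamping of its own to the result.
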(event Custom|UPorDown
  (bind _likedprogressbar (Variables|Default|GetLikedProgressBar))
  (if (Utilities|IsValid _likedprogressbar)
    (if (Variables|Default|GetisUp)
      (Progress|SetPercent _likedprogressbar (+ (Variables|/Script/UMG.ProgressBar|GetPercent _likedprogressbar) 0.1))
      (else
        (Progress|SetPercent _likedprogressbar (- (Variables|/Script/UMG.ProgressBar|GetPercent _likedprogressbar) 0.1))))))