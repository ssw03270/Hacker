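; TextBlock_BP is a temporary actor, likely a text panel by its name, that floats in front of the VR player's view.
; Every Tick it casts the player pawn to BP_VRPlayer_Man and places itself ahead of and slightly below the camera.
; It copies the camera's roll and pitch and turns the yaw half a turn to face back.
; A second Tick branch runs a Delay, destroying the actor about 18 seconds after ticking starts.
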(event EventBeginPlay)

(event Collision|EventActorBeginOverlap
  (params (OtherActor :type Actor%20Object%20Reference)))

(event EventTick
  (params (DeltaSeconds :type Float%20%28single-precision%29))
  (Utilities|FlowControl|Sequence
    (:then_0
      (bind _asbp_vrplayer_man (Utilities|Casting|CastToBP_VRPlayer_Man (Game|Player|GetPlayerPawn 0)))
      (Transformation|SetActorLocation (+ (Transformation|GetWorldLocation (Variables|/Game/vrpawn/blueprint/BP_VRPlayer_Man.BP_VRPlayer_Man_C|GetCamera _asbp_vrplayer_man)) (* (Math|Vector|GetForwardVector (Variables|/Game/vrpawn/blueprint/BP_VRPlayer_Man.BP_VRPlayer_Man_C|GetCamera _asbp_vrplayer_man)) 2e+02) (* (Math|Vector|GetUpVector (Variables|/Game/vrpawn/blueprint/BP_VRPlayer_Man.BP_VRPlayer_Man_C|GetCamera _asbp_vrplayer_man)) -3e+01)) false false)
      (Transformation|SetActorRotation (Math|Rotator|MakeRotator (.Roll (Math|Rotator|BreakRotator (Transformation|GetWorldRotation (Variables|/Game/vrpawn/blueprint/BP_VRPlayer_Man.BP_VRPlayer_Man_C|GetCamera _asbp_vrplayer_man)))) (.Pitch (Math|Rotator|BreakRotator (Transformation|GetWorldRotation (Variables|/Game/vrpawn/blueprint/BP_VRPlayer_Man.BP_VRPlayer_Man_C|GetCamera _asbp_vrplayer_man)))) (- (.Yaw (Math|Rotator|BreakRotator (Transformation|GetWorldRotation (Variables|/Game/vrpawn/blueprint/BP_VRPlayer_Man.BP_VRPlayer_Man_C|GetCamera _asbp_vrplayer_man)))) 1.8e+02))))
    (:then_1
      (Utilities|FlowControl|Delay 18.0)
      (Actor|DestroyActor))))

(fn ConstructionScript)